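; BP_Camera is a security camera actor that catches the first-person player and sends them back to a respawn point.
; On BeginPlay it spawns a BP_Respawn at a hard-coded location and stores it.
; When PawnSensing sees the player, it destroys the character and plays the DeadCamera_WD widget animation.
; It then immediately spawns a new character at the stored respawn transform and has player controller 0 possess it.
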(event `self.ReceiveBeginPlay`
  (bind _output_get (set `self.RespawnLocation` (-115.537469 -23.958284 413.02252)))
  (bind _returnvalue (`|SpawnActorFromClass` "/Game/Level1GDW/Level1Assets/Triggers/BP_Respawn.BP_Respawn_C" (`KismetMathLibrary.Conv_VectorToTransform` _output_get) "Undefined" "MultiplyWithRoot" null null))
  (set `self.Spawn` _returnvalue))

(event `self.PawnSensing.OnSeePawn`
  (params (Pawn :type "Pawn Object Reference"))
  (bind _asbp_first_person_character (cast `/Game/FirstPerson/Blueprints/BP_FirstPersonCharacter` Pawn))
  (`self.K2_DestroyActor` _asbp_first_person_character)
  (bind _returnvalue (`|CreateWidget` "/Game/Level1GDW/Level1Assets/Camera/DeadCamera_WD.DeadCamera_WD_C"))
  (`UserWidget.AddToViewport` _returnvalue 0)
  (`UserWidget.PlayAnimation` _returnvalue (`/Game/Level1GDW/Level1Assets/Camera/DeadCamera_WD.CamAnim` _returnvalue) 0.0 1 "Forward" 1.0 false)
  (`GameplayStatics.GetAllActorsOfClass` "/Game/Level1GDW/Level1Assets/Triggers/BP_Respawn.BP_Respawn_C")
  (bind _returnvalue_2 (`|SpawnActorFromClass` "/Game/FirstPerson/Blueprints/BP_FirstPersonCharacter.BP_FirstPersonCharacter_C" (`self.GetTransform` (`self.Spawn`)) "Undefined" "MultiplyWithRoot" null null))
  (`Controller.Possess` (`GameplayStatics.GetPlayerController` 0) _returnvalue_2))

(fn `UserConstructionScript`)