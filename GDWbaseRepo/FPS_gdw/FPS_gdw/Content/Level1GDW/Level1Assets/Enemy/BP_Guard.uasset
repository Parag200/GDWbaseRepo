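; BP_Guard is an enemy guard that wanders randomly and sends the first-person player back to a respawn point on sight.
; On BeginPlay it spawns a BP_Respawn at a hardcoded location and starts a wander loop, chaining AIMoveTo to random nearby navigable points after each success.
; PawnSensing destroys a seen player, spawns a replacement at that respawn actor and possesses it.
; A Hit event destroys the guard.
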(event `self.ReceiveBeginPlay`
  (`|ExecutionSequence`
    (:`then_0`
      (bind _output_get (set `self.RespawnLocation` (-115.537469 -23.958284 413.02252)))
      (bind _returnvalue (`|SpawnActorFromClass` "/Game/Level1GDW/Level1Assets/Triggers/BP_Respawn.BP_Respawn_C" (`KismetMathLibrary.Conv_VectorToTransform` _output_get) "Undefined" "MultiplyWithRoot" null null))
      (set `self.Spawn` _returnvalue))
    (:`then_1`
      (`self.MoveTo`))))

(event `MoveTo`
  (bind _randomlocation (`NavigationSystemV1.K2_GetRandomLocationInNavigableRadius` (`self.K2_GetActorLocation`) 1000.0 null null))
  (`|AIMoveTo` self _randomlocation null
    (:`OnSuccess`
      (`self.MoveTo`))))

(event `self.ReceiveHit`
  (params (MyComp :type "PrimitiveComponent Object Reference") (Other :type "Actor Object Reference") (OtherComp :type "PrimitiveComponent Object Reference") (bSelfMoved :type Boolean) (HitLocation :type "Vector Structure") (HitNormal :type "Vector Structure") (NormalImpulse :type "Vector Structure") (Hit :type "HitResult Structure (by ref)"))
  (`self.K2_DestroyActor`))

(event `self.PawnSensing.OnSeePawn`
  (params (Pawn :type "Pawn Object Reference"))
  (bind _asbp_first_person_character (cast `/Game/FirstPerson/Blueprints/BP_FirstPersonCharacter` Pawn))
  (`self.K2_DestroyActor` _asbp_first_person_character)
  (`GameplayStatics.GetAllActorsOfClass` "/Game/Level1GDW/Level1Assets/Triggers/BP_Respawn.BP_Respawn_C")
  (bind _returnvalue (`|SpawnActorFromClass` "/Game/FirstPerson/Blueprints/BP_FirstPersonCharacter.BP_FirstPersonCharacter_C" (`self.GetTransform` (`self.Spawn`)) "Undefined" "MultiplyWithRoot" null null))
  (`Controller.Possess` (`GameplayStatics.GetPlayerController` 0) _returnvalue))

(fn `UserConstructionScript`)