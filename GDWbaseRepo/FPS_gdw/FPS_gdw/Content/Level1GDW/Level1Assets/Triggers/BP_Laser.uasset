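; BP_Laser is a lethal laser hazard in Level 1 that reacts to actor overlaps.
; An overlapping first-person character is destroyed, and the DeadLaser_WD death widget appears and plays its laser animation.
; A fresh character then spawns at the Spawn reference's transform and is possessed by player controller 0; the BP_Respawn lookup's result goes unused.
; Overlapping teleport darts are also destroyed.
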(event `self.ReceiveActorBeginOverlap`
  (params (OtherActor :type "Actor Object Reference"))
  (`|ExecutionSequence`
    (:`then_0`
      (bind _asbp_first_person_character (cast `/Game/FirstPerson/Blueprints/BP_FirstPersonCharacter` OtherActor))
      (`self.K2_DestroyActor` _asbp_first_person_character)
      (bind _returnvalue (`|CreateWidget` "/Game/Level1GDW/DeadWidgets/DeadLaser_WD.DeadLaser_WD_C"))
      (`UserWidget.AddToViewport` _returnvalue 0)
      (`UserWidget.PlayAnimation` _returnvalue (`/Game/Level1GDW/DeadWidgets/DeadLaser_WD.LaserAnim` _returnvalue) 0.0 1 "Forward" 1.0 false)
      (`GameplayStatics.GetAllActorsOfClass` "/Game/Level1GDW/Level1Assets/Triggers/BP_Respawn.BP_Respawn_C")
      (bind _returnvalue_2 (`|SpawnActorFromClass` "/Game/FirstPerson/Blueprints/BP_FirstPersonCharacter.BP_FirstPersonCharacter_C" (`self.GetTransform` (`self.Spawn`)) "Undefined" "MultiplyWithRoot" null null))
      (`Controller.Possess` (`GameplayStatics.GetPlayerController` 0) _returnvalue_2))
    (:`then_1`
      (bind _asbp_teleport_dart (cast `/Game/Level1GDW/Level1Assets/Guns/TeleportGun/BP_TeleportDart` OtherActor))
      (`self.K2_DestroyActor` _asbp_teleport_dart))))

(fn `SPAWNPOINT`)

(fn `UserConstructionScript`)